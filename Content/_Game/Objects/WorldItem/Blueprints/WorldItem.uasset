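; WorldItem is a base pickup actor that hovers in the world and reacts when a TopDownCharacter overlaps it.
; The construction script sizes the collision sphere and keeps either the static mesh or the Niagara effect.
; A self-restarting timeline drives height and yaw offsets from the captured transform.
; On overlap, a valid InteractAudio plays and gates the call to OnInteract, an empty hook receiving the player.
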(event `self.ReceiveBeginPlay`
  (`self.Hover Item`))

(event `Hover Item`
  (bind _origin (`self.Origin`))
  (set `self.Origin` (`SceneComponent.K2_GetComponentToWorld` (`self.DefaultSceneRoot`)))
  (bind (_direction _z_position _z_rotation) (`Timeline|Hover` :!via `PlayFromStart`)
    (:`Update`
      (`|ExecutionSequence`
        (:`then_0`
          (`SceneComponent.K2_SetWorldLocation` (`self.DefaultSceneRoot`) (`KismetMathLibrary.MakeVector` (.x (.location _origin)) (.y (.location _origin)) (+ (.z (.location _origin)) _z_position)) false false))
        (:`then_1`
          (`SceneComponent.K2_SetWorldRotation` (`self.DefaultSceneRoot`) (`KismetMathLibrary.MakeRotator` (.roll (.rotation _origin)) (.pitch (.rotation _origin)) (+ _z_rotation (.yaw (.rotation _origin)))) false false))))
    (:`Finished`
      (`self.Hover Item`))))

(event `self.ReceiveActorBeginOverlap`
  (params (OtherActor :type "Actor Object Reference"))
  (bind _astop_down_character (cast `/Game/_Game/Objects/Player/Blueprints/TopDownCharacter` OtherActor))
  (bind _interact_audio (`self.Interact Audio`)
    (:`then`
      (`GameplayStatics.PlaySoundAtLocation` _interact_audio (`self.K2_GetActorLocation`) (struct) 1.0 1.0 0.0 null null null)
      (`self.On Interact` _astop_down_character))
    (:`else`)))

(fn `On Interact`
  (params (Player :type "/Game/_Game/Objects/Player/Blueprints/TopDownCharacter Object Reference")))

(fn `UserConstructionScript`
  (`SphereComponent.SetSphereRadius` (`self.Sphere Collision`) (`self.Overlap Radius`) true)
  (if (`self.Use Niagara Effect`)
    (`ActorComponent.K2_DestroyComponent` (`self.Static Mesh`))
    (else
      (`ActorComponent.K2_DestroyComponent` (`self.Niagara Effect`)))))