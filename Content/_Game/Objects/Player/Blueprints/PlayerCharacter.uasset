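; Player character Blueprint that handles health regeneration and a two-slot weapon inventory.
; Tick calls a regeneration function that, when enabled, adds health scaled by delta time, though its check passes only at or above MaxHealth.
; Pick Up Weapon stores the world item's class in the first empty slot, or replaces the currently selected slot when both are full.
; An unconnected sphere overlap for nearby weapon items never runs.
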(event `self.ReceiveTick`
  (params (DeltaSeconds :type "Float (single-precision)"))
  (`parent.ReceiveTick` DeltaSeconds)
  (`|ExecutionSequence`
    (:`then_0`
      (if (`self.Can Regenerate Health`)
        (if (>= (`self.Health`) (`self.Max Health`))
          (set `self.Health` (+ (`self.Health`) (* (`self.Health Regen Rate`) DeltaSeconds))))))))

(fn `Pick Up Weapon`
  (params (`World Item` :type "/Game/_Game/Objects/Weapons/Blueprints/WI_Weapon Object Reference"))
  (bind (_weapons_slot1 _weapons_slot2) (break `/Game/_Game/Objects/Player/Structs/S_WeaponSlots` (`self.Weapons`)))
  (bind (_weapons_slot1_2 _weapons_slot2_2) (break `/Game/_Game/Objects/Player/Structs/S_WeaponSlots` (`self.Weapons`)))
  (bind _weapons_slot1_3 (break `/Game/_Game/Objects/Player/Structs/S_WeaponSlots` (`self.Weapons`)))
  (bind (_weapons_slot1_4 _weapons_slot2_3) (break `/Game/_Game/Objects/Player/Structs/S_WeaponSlots` (`self.Weapons`)))
  (bind _class (`/Game/_Game/Objects/Weapons/Blueprints/WI_Weapon.Class` `World Item`))
  (bind _weapons_slot1_5 (break `/Game/_Game/Objects/Player/Structs/S_WeaponSlots` (`self.Weapons`)))
  (bind (_weapons_slot1_6 _weapons_slot2_4) (break `/Game/_Game/Objects/Player/Structs/S_WeaponSlots` (`self.Weapons`)))
  (if (and (`KismetSystemLibrary.IsValidClass` _weapons_slot1_2) (`KismetSystemLibrary.IsValidClass` _weapons_slot2_2))
    (set `self.Weapons` (select `int` (`self.Current Weapon Index`) :`0` (make `/Game/_Game/Objects/Player/Structs/S_WeaponSlots` _class _weapons_slot2) :`1` (make `/Game/_Game/Objects/Player/Structs/S_WeaponSlots` _weapons_slot1 _class) :!type "/Game/_Game/Objects/Player/Structs/S_WeaponSlots Structure"))
    (elif (not (`KismetSystemLibrary.IsValidClass` _weapons_slot1_3))
      (set `self.Weapons` (make `/Game/_Game/Objects/Player/Structs/S_WeaponSlots` (`/Game/_Game/Objects/Weapons/Blueprints/WI_Weapon.Class` (`local.World Item`)) _weapons_slot2_3))
      (elif (not (`KismetSystemLibrary.IsValidClass` _weapons_slot2_4))
        (set `self.Weapons` (make `/Game/_Game/Objects/Player/Structs/S_WeaponSlots` _weapons_slot1_5 (`/Game/_Game/Objects/Weapons/Blueprints/WI_Weapon.Class` (`local.World Item`))))))))

(fn `UserConstructionScript`
  (`parent.UserConstructionScript`))